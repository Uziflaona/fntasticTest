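; BP_btn2 is a clickable button actor that spawns a BP_TurtlePig2 with a smoke effect.
; Clicking plays a press sound, pushes the Sphere against Direction by Stroke, spawns BP_Smoke at TortleSpawnTransform, then spawns the turtle pig there after a short delay.
; Releasing plays a release sound and moves the Sphere back by the same offset.
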(event EventBeginPlay)

(event Collision|EventActorBeginOverlap
  (params (OtherActor :type Actor%20Object%20Reference)))

(event EventTick
  (params (DeltaSeconds :type Float%20%28single-precision%29)))

(event EventActorOnReleased
  (params (ButtonReleased :type Key%20Structure :default "None"))
  (Audio|PlaySound2D "/Game/SFX/CUE_BtnRelesed.CUE_BtnRelesed" 1.0 1.0 0.0 0 0)
  ;[1 1 1] Click_Display
  (Transformation|AddWorldOffset (Variables|Default|GetSphere) (* (Variables|Default|Getdirection) (Variables|Default|Getstroke)) false false))

(event MouseInput|EventActorOnClicked
  (params (ButtonPressed :type Key%20Structure :default "None"))
  (Audio|PlaySound2D "/Game/SFX/CUE_BtnPressed.CUE_BtnPressed" 1.0 1.0 0.0 0 0)
  ;[1 1 1] Click_Display
  (Transformation|AddWorldOffset (Variables|Default|GetSphere) (* (Variables|Default|Getdirection) (* (Variables|Default|Getstroke) -1.0)) false false)
  ;[1 1 1] Create Turtles
  (Game|SpawnActorfromClass "/Game/Blueprints/Constructions/Pig/BP_Smoke.BP_Smoke_C" (Variables|Default|GetTortle_spawn_transform) "Undefined" 0 0)
  (Utilities|FlowControl|Delay 2.0)
  (Game|SpawnActorfromClass "/Game/Blueprints/Constructions/Pig/BP_TurtlePig2.BP_TurtlePig2_C" (Variables|Default|GetTortle_spawn_transform) "Undefined" 0 0))

(fn ConstructionScript
  (|CallParentFunction))