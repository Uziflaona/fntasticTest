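; BP_TurtlePig2 is a pig construction actor that alternates between walking and standing, switching about once a second.
; Tick switches on Selection: walking calls Walk2 and offsets the skeletal mesh by Speed times Direction each frame, standing calls Stop2.
; Delays flip the state and stop or play the Steps audio component added at BeginPlay.
; Any actor overlap spawns BP_Smoke in its place and destroys it.
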(event Collision|EventActorBeginOverlap
  (params (OtherActor :type Actor%20Object%20Reference))
  ;[1 1 1] Destroy
  (Game|SpawnActorfromClass "/Game/Blueprints/Constructions/Pig/BP_Smoke.BP_Smoke_C" (Transformation|GetActorTransform) "Undefined" 0 0)
  (Actor|DestroyActor))

(event EventBeginPlay
  (bind _returnvalue (AddComponent|AddAudioComponent false))
  (Variables|Default|SetSteps _returnvalue))

(event EventTick
  (params (DeltaSeconds :type Float%20%28single-precision%29))
  (switch int (Variables|Default|GetSelection)
    (:0
      ;[1 1 1] Walking
      (CallFunction|Walk)
      (Utilities|FlowControl|Delay 1.0)
      (Variables|Default|SetSelection 1)
      (Audio|Components|Audio|Stop (Variables|Default|GetSteps)))
    (:1
      ;[1 1 1] Standing
      (Default|CallStop2)
      (Utilities|FlowControl|Delay 1.0)
      (Variables|Default|SetSelection 0)
      (Audio|Components|Audio|Play (Variables|Default|GetSteps) 0.0))))

(fn ConstructionScript)

(fn Walk
  (Default|CallWalk2)
  (Transformation|AddWorldOffset (Variables|Default|GetSkeletalMesh) (* (Variables|Default|GetSpeed) (Variables|Default|GetDirection)) false false))