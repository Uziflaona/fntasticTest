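; BP_TurtlePig is a moving pig actor that vanishes in smoke when it overlaps another actor.
; It adds an audio component on BeginPlay, then offsets its skeletal mesh by Speed times Direction every tick, without sweep or delta-time scaling.
; Any overlap, with no filtering, spawns BP_Smoke at the actor's transform and destroys the pig.
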(event EventBeginPlay
  (AddComponent|AddAudioComponent false))

(event Collision|EventActorBeginOverlap
  (params (OtherActor :type Actor%20Object%20Reference))
  (Game|SpawnActorfromClass "/Game/Blueprints/Constructions/Pig/BP_Smoke.BP_Smoke_C" (Transformation|GetActorTransform) "Undefined" 0 0)
  (Actor|DestroyActor))

(event EventTick
  (params (DeltaSeconds :type Float%20%28single-precision%29))
  (Transformation|AddWorldOffset (Variables|Default|GetSkeletalMesh) (* (Variables|Default|GetSpeed) (Variables|Default|GetDirection)) false false))

(fn ConstructionScript)