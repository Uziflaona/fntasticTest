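; Turtle pig actor that shuffles forward and back, and turns into a puff of smoke when any actor overlaps it.
; Tick switches on Selection to offset the skeletal mesh along Direction by Speed, with looping Delays alternating longer forward and shorter backward phases.
; Each step calls Walk3 or GoBack3, and movement is unswept and not scaled by delta time.
; BeginPlay adds an audio component; overlap spawns BP_Smoke and destroys the actor.
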(event Collision|EventActorBeginOverlap
  (params (OtherActor :type Actor%20Object%20Reference))
  (Game|SpawnActorfromClass "/Game/Blueprints/Constructions/Pig/BP_Smoke.BP_Smoke_C" (Transformation|GetActorTransform) "Undefined" 0 0)
  (Actor|DestroyActor))

(event EventTick
  (params (DeltaSeconds :type Float%20%28single-precision%29))
  (switch int (Variables|Default|GetSelection) :!label _label
    (:0
      ;[1 1 1] Walking
      (CallFunction|Walk)
      (Utilities|FlowControl|Delay 1.0)
      (Variables|Default|SetSelection 1)
      (goto _label))
    (:1
      ;[1 1 1] WalkingBack
      (CallFunction|WalkBack)
      (Utilities|FlowControl|Delay 0.5)
      (Variables|Default|SetSelection 0)
      (goto _label))))

(event EventBeginPlay
  (AddComponent|AddAudioComponent false))

(fn ConstructionScript)

(fn Walk
  (Default|CallWalk3)
  (Transformation|AddWorldOffset (Variables|Default|GetSkeletalMesh) (* (Variables|Default|GetSpeed) (Variables|Default|GetDirection)) false false))

(fn WalkBack
  (Default|CallGoBack3)
  (Transformation|AddWorldOffset (Variables|Default|GetSkeletalMesh) (* (* (Variables|Default|GetSpeed) -1.0) (Variables|Default|GetDirection)) false false))